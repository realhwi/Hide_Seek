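; VR game instance Blueprint that manages multiplayer sessions, map travel and the lobby UI.
; It creates a two-connection session using a toggleable LAN flag, then opens TestMap as a listen server; joining only prints success or failure.
; Map travel stores the connected player count and runs a serverTravel console command.
; The main menu creates and caches the lobby widget, then switches to UI-only input with a visible cursor.
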(event `CreateGameSession`
  (`CreateSessionCallbackProxy.CreateSession` (`GameplayStatics.GetPlayerController` 0) 2 (`self.isLanConnect`)
    (:`then`
      (`GameplayStatics.OpenLevel` "TestMap" true "?listen"))))

(event `JoinGameSession`
  (params (SessionResult :type "BlueprintSessionResult Structure"))
  (`JoinSessionCallbackProxy.JoinSession` (`GameplayStatics.GetPlayerController` 0) SessionResult
    (:`OnSuccess`
      (`KismetSystemLibrary.PrintString` "success"))
    (:`OnFailure`
      (`KismetSystemLibrary.PrintString` "fail"))))

(event `TravelToMap`
  (params (NumConnectedPlayers :type Integer) (MapName :type String))
  (set `self.Num Connected Players` NumConnectedPlayers)
  (`KismetSystemLibrary.ExecuteConsoleCommand` (`KismetStringLibrary.Concat_StrStr` "serverTravel " MapName) (`GameplayStatics.GetPlayerController` 0)))

(fn `ChangeConnectionType`
  (returns (IsLanGame :type Boolean))
  (if (`self.isLanConnect`)
    (set `self.isLanConnect` false)
    (else
      (set `self.isLanConnect` true)))
  (return (`self.isLanConnect`)))

(fn `ShowMainMenu`
  (bind _returnvalue (`GameplayStatics.GetPlayerController` 0))
  (`/Engine/EditorBlueprintResources/StandardMacros.IsValid` (`self.LobbyUIRef`)
    (:`Is Valid`
      _)
    (:`Is Not Valid`
      (bind _returnvalue_2 (`|CreateWidget` "/Game/Mandol/UI/LobbyUI/WBP_VRLobbyUI.WBP_VRLobbyUI_C" _returnvalue))
      (set `self.LobbyUIRef` _returnvalue_2)))
  (`UserWidget.AddToViewport` (`self.LobbyUIRef`) 0)
  (`WidgetBlueprintLibrary.SetInputMode_UIOnlyEx` _returnvalue null)
  (set `PlayerController.bShowMouseCursor` true _returnvalue)
  (return))