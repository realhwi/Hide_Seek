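; Player controller for the lobby, which sets up UI-only input and handles session menu and teardown.
; On begin play the local controller shows the mouse cursor and switches input to UI only.
; A menu event creates the VR session widget once, caches it and adds it to the viewport.
; Ending a client session destroys the session and, on completion, reopens the LobbyMap level.
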(event `self.ReceiveBeginPlay`
  (if (`self.IsLocalController`)
    (set `self.bShowMouseCursor` true)
    (`WidgetBlueprintLibrary.SetInputMode_UIOnlyEx` self null)))

(event `EndClientSession`
  (`DestroySessionCallbackProxy.DestroySession` self
    (:`then`
      (`GameplayStatics.OpenLevel` "LobbyMap"))))

(event `CreateSessionMenu`
  (`self.UIShowSessionMenu`))

(fn `UIShowSessionMenu`
  (`/Engine/EditorBlueprintResources/StandardMacros.IsValid` (`self.WBP_VRSessionUIRef`)
    (:`Is Valid`
      _)
    (:`Is Not Valid`
      (bind _returnvalue (`|CreateWidget` "/Game/Mandol/UI/LobbyUI/WBP_VRSessionUI.WBP_VRSessionUI_C" self))
      (set `self.WBP_VRSessionUIRef` _returnvalue)))
  (`UserWidget.AddToViewport` (`self.WBP_VRSessionUIRef`) 0)
  (return))

(fn `UserConstructionScript`)