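; BP_VRPlayerController is a player controller that sets up game input and a game-mode UI for the local player.
; On BeginPlay, marked "Not Use", it switches to game-only input, hides the cursor and adds WBP_GameModeUI to the viewport with a countdown.
; An unconnected chain removes widgets and prints a debug message based on a BP_TESTSPawnGMB game mode flag; Tick and the construction script are empty.
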(event `self.ReceiveBeginPlay`
  ;[1 1 1] Not Use
  (if (`self.IsLocalPlayerController`)
    (`WidgetBlueprintLibrary.SetInputMode_GameOnly` self)
    (set `self.bShowMouseCursor` false)
    (bind _returnvalue (`|CreateWidget` "/Game/Mandol/UI/WBP_GameModeUI.WBP_GameModeUI_C"))
    (`UserWidget.AddToViewport` _returnvalue 0)))

(fn `UserConstructionScript`)