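; VR enemy player character that feeds camera and motion controller transforms to its animation blueprint each tick.
; Pressing interact sphere-traces to damage a player for an HP chip, or find a door, item box or altar.
; Holding it counts down door destruction, adds item box lock time with skill one, or deposits chips.
; A timer accumulates skill time, but skill activation logic is disconnected, leaving only debug-print checks.
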(event `self.ReceiveBeginPlay`
  (`self.SetSkillTime`))

(event `AttachHudOnHand`)

(event `self.ReceiveTick`
  (params (DeltaSeconds :type "Float (single-precision)"))
  (`self.CheckSkillTime`)
  (bind _asabp_vrenemy_ub (cast `/Game/Mandol/Animations/ABP_VREnemyUB` (`SkeletalMeshComponent.GetAnimInstance` (`self.Mesh`))))
  (set `/Game/Mandol/Animations/ABP_VREnemyUB.HeadTransform` (`SceneComponent.K2_GetComponentToWorld` (`self.cameraComp`)) _asabp_vrenemy_ub)
  (set `/Game/Mandol/Animations/ABP_VREnemyUB.LeftHandTransform` (`SceneComponent.K2_GetComponentToWorld` (`self.leftMotionCtrl`)) _asabp_vrenemy_ub)
  (set `/Game/Mandol/Animations/ABP_VREnemyUB.RightHandTransform` (`SceneComponent.K2_GetComponentToWorld` (`self.rightMotionCtrl`)) _asabp_vrenemy_ub))

(event `EnhancedInput|/Game/Mandol/Input/Actions/IA_EnemyInteraction`
  (params (ActionValue :type Boolean) (ElapsedSeconds :type "Float (double-precision)") (TriggeredSeconds :type "Float (double-precision)") (InputAction :type "InputAction Object Reference" :default "/Game/Mandol/Input/Actions/IA_EnemyInteraction.IA_EnemyInteraction"))
  (bind _doorref (`self.DoorRef`))
  (bind _doorref_2 (`self.DoorRef`))
  (bind _itemboxref (`self.ItemBoxRef`))
  (bind _returnvalue (+ (`SceneComponent.K2_GetComponentLocation` (`self.Mesh`)) (0.0 0.0 50.0)))
  (bind _returnvalue_2 (+ (`SceneComponent.K2_GetComponentLocation` (`self.Mesh`)) (0.0 0.0 50.0)))
  (:`Triggered`
    (`|ExecutionSequence`
      (:`then_0`
        (`/Engine/EditorBlueprintResources/StandardMacros.IsValid` _doorref
          (:`Is Valid`
            (if (> (`/Game/Mandol/Blueprints/BP_Door.EnemyOpenTime` _doorref) 0.0)
              (set `/Game/Mandol/Blueprints/BP_Door.EnemyOpenTime` (- (`/Game/Mandol/Blueprints/BP_Door.EnemyOpenTime` _doorref) (`GameplayStatics.GetWorldDeltaSeconds`)) _doorref_2)
              (else
                (`self.K2_DestroyActor` _doorref_2))))))
      (:`then_1`
        (`/Engine/EditorBlueprintResources/StandardMacros.IsValid` _itemboxref
          (:`Is Valid`
            (if (`/Game/Mandol/Blueprints/BP_ItemBox.isOpen` _itemboxref)
              (`KismetSystemLibrary.PrintString` "Already Open!!!")
              (elif (`self.activeFirstSkill`)
                (if (`/Game/Mandol/Blueprints/BP_ItemBox.isLock` (`self.ItemBoxRef`))
                  (`KismetSystemLibrary.PrintString` "Already Lock!!!!")
                  (else
                    (set `/Game/Mandol/Blueprints/BP_ItemBox.IBOpenTime` (+ (`/Game/Mandol/Blueprints/BP_ItemBox.IBOpenTime` (`self.ItemBoxRef`)) (`KismetMathLibrary.FClamp` (`GameplayStatics.GetWorldDeltaSeconds`) 0.0 (`self.addIBLockTime`))) (`self.ItemBoxRef`))))
                (else
                  (`KismetSystemLibrary.PrintString` "Net Yet Active Skill")))))))
      (:`then_2`
        (`/Engine/EditorBlueprintResources/StandardMacros.IsValid` (`self.AltarRef`)
          (:`Is Valid`
            (if (and (`self.inAltar`) (> (`self.CountHPChip`) 0))
              (set `/Game/Mandol/Blueprints/BP_EnemyAltar.SetPlayerChip` (`self.CountHPChip`) (`self.AltarRef`))
              (set `self.CountHPChip` 0)
              (else
                (`KismetSystemLibrary.PrintString` "Nope!!!!"))))))))
  (:`Started`
    (bind (_outhit _returnvalue_3) (`KismetSystemLibrary.SphereTraceSingleForObjects` :`Start` _returnvalue_2 :`End` _returnvalue_2 :`Radius` 100.0 :`ObjectTypes` (`|MakeArray` "ObjectTypeQuery3" :!type "EObjectTypeQuery Enum") :`DrawDebugType` "ForDuration"))
    (if _returnvalue_3
      (bind (_bblockinghit _binitialoverlap _time _distance _location _impactpoint _normal _impactnormal _physmat _hitactor) (`GameplayStatics.BreakHitResult` _outhit))
      (if (`self.ActorHasTag` _hitactor "Player")
        (bind _asbp_test_player (cast `/Game/Mandol/Blueprints/BP_TestPlayer` _hitactor))
        (set `self.playerChar` _asbp_test_player)
        (bind _output_get (set `self.TestPlayerRef` _asbp_test_player))
        (set `/Game/Mandol/Blueprints/BP_TestPlayer.PlayerCurrentHP` (- (`/Game/Mandol/Blueprints/BP_TestPlayer.PlayerCurrentHP` _output_get) 1.0) _output_get)
        (set `self.CountHPChip` (+ (`self.CountHPChip`) 1)))
      (else
        (bind (_outhit_2 _returnvalue_4) (`KismetSystemLibrary.SphereTraceSingleForObjects` :`Start` _returnvalue :`End` _returnvalue :`Radius` 90.0 :`ObjectTypes` (`|MakeArray` "ObjectTypeQuery2" :!type "EObjectTypeQuery Enum") :`DrawDebugType` "ForDuration"))
        (if _returnvalue_4
          (bind (_bblockinghit_2 _binitialoverlap_2 _time_2 _distance_2 _location_2 _impactpoint_2 _normal_2 _impactnormal_2 _physmat_2 _hitactor_2) (`GameplayStatics.BreakHitResult` _outhit_2))
          (if (`self.ActorHasTag` _hitactor_2 "Door")
            (bind _asbp_door (cast `/Game/Mandol/Blueprints/BP_Door` _hitactor_2))
            (set `self.door` _asbp_door)
            (set `self.DoorRef` _asbp_door)
            (elif (`self.ActorHasTag` _hitactor_2 "ItemBox")
              (bind _asbp_item_box (cast `/Game/Mandol/Blueprints/BP_ItemBox` _hitactor_2))
              (set `self.itemBox` _asbp_item_box)
              (set `self.ItemBoxRef` _asbp_item_box)
              (elif (`self.ActorHasTag` _hitactor_2 "Altar")
                (bind _asbp_enemy_altar (cast `/Game/Mandol/Blueprints/BP_EnemyAltar` _hitactor_2))
                (set `self.enemyAltar` _asbp_enemy_altar)
                (set `self.AltarRef` _asbp_enemy_altar)
                (set `self.inAltar` true))))))))
  (:`Completed`
    (set `self.playerChar` null)
    (set `self.TestPlayerRef` null)
    (set `self.door` null)
    (set `self.DoorRef` null)
    (set `self.itemBox` null)
    (set `self.ItemBoxRef` null)
    (set `self.enemyAltar` null)
    (set `self.AltarRef` null)
    (set `self.inAltar` false)))

(event `SetSkillTime`
  (bind _activemaxskilltime (`self.activeMaxSkillTime`))
  (bind _output_get (set `self.activeSkillTime` (`KismetMathLibrary.FClamp` (+ (`self.activeSkillTime`) 1.0) 0.0 _activemaxskilltime)))
  (if (== _output_get _activemaxskilltime)
    (`KismetSystemLibrary.K2_ClearAndInvalidateTimerHandle` (stale _returnvalue))
    (else
      (bind _returnvalue (`KismetSystemLibrary.K2_SetTimerDelegate` (delegate `SetSkillTime`) 1.0)))))

(event `FirstSkillOn`
  (if (`self.activeFirstSkill`)
    (`/Engine/EditorBlueprintResources/StandardMacros.DoOnce` false
      (:`Completed`
        (`KismetSystemLibrary.PrintString` "FirstON!!!")))))

(event `SecondSkillOn`
  (if (`self.activeSecondSkill`)
    (`/Engine/EditorBlueprintResources/StandardMacros.DoOnce` false
      (:`Completed`
        (`KismetSystemLibrary.PrintString` "SecondON!!!")))))

(event `ThirdSkillOn`
  (if (`self.activeThirdSkill`)
    (`/Engine/EditorBlueprintResources/StandardMacros.DoOnce` false
      (:`Completed`
        (`KismetSystemLibrary.PrintString` "ThirdON!!!")))))

(event `CheckSkillTime`
  (`self.FirstSkillOn`)
  (`self.SecondSkillOn`)
  (`self.ThirdSkillOn`))

(fn `UserConstructionScript`)