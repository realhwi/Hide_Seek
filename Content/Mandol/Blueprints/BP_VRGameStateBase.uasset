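; VR game state that shows the game mode UI and counts down play time once the enemy player joins.
; BeginPlay finds the BP_VREnemyPlayer actor and adds a WBP_GameModeUI widget with its own fixed starting countdown.
; Tick polls that actor's JoinEnemyPlayer flag without a validity check and, while true, lowers CountPlayTime toward zero.
; CountPlayTime is not passed to the widget here, and the node setting IsStartCountdown is unconnected.
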(event `self.ReceiveBeginPlay`
  (bind _returnvalue (`GameplayStatics.GetActorOfClass` "/Game/Mandol/Blueprints/BP_VREnemyPlayer.BP_VREnemyPlayer_C"))
  (set `self.VREemyRef` _returnvalue)
  (bind _returnvalue_2 (`|CreateWidget` "/Game/Mandol/UI/WBP_GameModeUI.WBP_GameModeUI_C"))
  (`UserWidget.AddToViewport` _returnvalue_2 0))

(event `self.ReceiveTick`
  (params (DeltaSeconds :type "Float (single-precision)"))
  (if (`VREnemyPlayer.joinEnemyPlayer` (`self.VREemyRef`))
    (set `self.countPlayTime` (`KismetMathLibrary.FClamp` (- (`self.countPlayTime`) DeltaSeconds) 0.0 (`self.countPlayTime`)))))

(fn `UserConstructionScript`)