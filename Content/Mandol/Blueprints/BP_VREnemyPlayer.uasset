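; VR enemy player character that wins by praying at an altar to place three HP chips, or when the game state's time runs out.
; An interaction input runs a five-second, input-locked pray that spends a chip.
; Tick polls altar chips, timeout and skill icons, showing the win UI where remote role is Authority.
; A one-second timer counts skill time, but skill activation, chip gain, lose UI and VR body-tracking logic are disconnected.
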(event `SetSkillTime`
  (bind _activemaxskilltime (`self.activeMaxSkillTime`))
  ;[1 1 1] SetSkill
  (bind _output_get (set `self.activeSkillTime` (`KismetMathLibrary.FClamp` (+ (`self.activeSkillTime`) 1.0) 0.0 _activemaxskilltime)))
  (if (== _output_get _activemaxskilltime)
    (`KismetSystemLibrary.K2_ClearAndInvalidateTimerHandle` (stale _returnvalue))
    (else
      (bind _returnvalue (`KismetSystemLibrary.K2_SetTimerDelegate` (delegate `SetSkillTime`) 1.0)))))

(event `self.ReceiveBeginPlay`
  (`self.SetSkillTime`)
  ;[1 1 1] EnemyHUD
  (bind _returnvalue (`|CreateWidget` "/Game/Mandol/UI/EnemyUI/WBP_EnemyHUD.WBP_EnemyHUD_C"))
  (bind _output_get (set `self.EnemyHUDRef` _returnvalue))
  (`UserWidget.AddToViewport` _output_get 0)
  (`Widget.SetVisibility` _returnvalue "Hidden")
  (if (`|EnumEquality` (`self.GetRemoteRole` (`self.GetOwner`)) "ROLE_Authority")
    (`/Engine/EditorBlueprintResources/StandardMacros.IsValid` _returnvalue
      (:`Is Valid`
        (`Widget.SetVisibility` _returnvalue "Visible")
        ;[1 1 1] EnemyWinUI
        (bind _returnvalue_2 (`|CreateWidget` "/Game/Mandol/UI/EnemyUI/WBP_EnemyWinUI.WBP_EnemyWinUI_C"))
        (bind _output_get_2 (set `self.EnemyWinRef` _returnvalue_2))
        (`UserWidget.AddToViewport` _output_get_2 0)
        (`Widget.SetVisibility` _returnvalue_2 "Collapsed")
        ;[1 1 1] EnemyLoseUI
        (bind _returnvalue_3 (`|CreateWidget` "/Game/Mandol/UI/EnemyUI/WBP_EnemyLoseUI.WBP_EnemyLoseUI_C"))
        (bind _output_get_3 (set `self.EnemyLoseRef` _returnvalue_3))
        (`UserWidget.AddToViewport` _output_get_3 0)
        (`Widget.SetVisibility` _returnvalue_3 "Collapsed")
        (bind _asbp_vrgame_state_base (cast `/Game/Mandol/Blueprints/BP_VRGameStateBase` (`GameplayStatics.GetGameState`)))
        (set `self.vrGameStateBase` _asbp_vrgame_state_base)))))

(event `EnhancedInput|/Game/Mandol/Input/Actions/IA_EnemyInteraction`
  (params (ActionValue :type Boolean) (ElapsedSeconds :type "Float (double-precision)") (TriggeredSeconds :type "Float (double-precision)") (InputAction :type "InputAction Object Reference" :default "/Game/Mandol/Input/Actions/IA_EnemyInteraction.IA_EnemyInteraction"))
  ;[1 1 1] Comment
  (:`Started`
    (if (`self.inAltar`)
      (if (> (`self.countHPChip`) 0)
        (`self.OnPrayAinm`)
        (`self.DisableInput` (`GameplayStatics.GetPlayerController` 0))
        (`KismetSystemLibrary.Delay` 5.0)
        (set `self.setAltarOnChip` (+ (`self.setAltarOnChip`) 1))
        (set `self.countHPChip` (- (`self.countHPChip`) 1))
        (`self.EnableInput` (`GameplayStatics.GetPlayerController` 0))
        (`self.OffPrayAnim`)))))

(event `self.ReceiveActorBeginOverlap`
  (params (OtherActor :type "Actor Object Reference"))
  ;[1 1 1] Altar Overlap
  (if (`self.ActorHasTag` OtherActor "Altar")
    (bind _asbp_enemy_altar (cast `/Game/Mandol/Blueprints/BP_EnemyAltar` OtherActor))
    (set `self.AltarRef` _asbp_enemy_altar)
    (set `self.inAltar` true)))

(event `CheckAltarOnChip`
  ;[1 1 1] Comment
  (switch `int` (`self.setAltarOnChip`)
    (:`1`
      (`SceneComponent.SetVisibility` (`/Game/Mandol/Blueprints/BP_EnemyAltar.HPChip1` (`self.AltarRef`)) true false))
    (:`2`
      (`SceneComponent.SetVisibility` (`/Game/Mandol/Blueprints/BP_EnemyAltar.HPChip2` (`self.AltarRef`)) true false))
    (:`3`
      (`SceneComponent.SetVisibility` (`/Game/Mandol/Blueprints/BP_EnemyAltar.HPChip3` (`self.AltarRef`)) true false)
      (set `self.isAltarActivate` true)
      (`self.checkEnemyWin`)
      (`KismetSystemLibrary.PrintString` "Win!!!!!"))))

(event `OnSkillIcon`
  ;[1 1 1] Skill UI On
  (`|ExecutionSequence`
    (:`then_0`
      (if (`self.activeFirstSkill`)
        (set `Widget.Visibility` "Visible" (`/Game/Mandol/UI/EnemyUI/WBP_EnemyHUD.Img_skillOne` (`self.EnemyHUDRef`)))))
    (:`then_1`
      (if (`self.activeSecondSkill`)
        (set `Widget.Visibility` "Visible" (`/Game/Mandol/UI/EnemyUI/WBP_EnemyHUD.Img_skillTwo` (`self.EnemyHUDRef`)))))
    (:`then_2`
      (if (`self.activeThirdSkill`)
        (set `Widget.Visibility` "Visible" (`/Game/Mandol/UI/EnemyUI/WBP_EnemyHUD.Img_skillThree` (`self.EnemyHUDRef`)))))))

(event `self.ReceiveActorEndOverlap`
  (params (OtherActor :type "Actor Object Reference"))
  ;[1 1 1] Altar Overlap
  (if (`self.ActorHasTag` OtherActor "Altar")
    (set `self.inAltar` false)))

(event `OnPrayAinm`
  ;[1 1 1] Comment
  (set `self.isPraying` true))

(event `OffPrayAnim`
  ;[1 1 1] Comment
  (set `self.isPraying` false)
  (set `self.isHandUP` false))

(event `self.ReceiveTick`
  (params (DeltaSeconds :type "Float (single-precision)"))
  (bind _returnvalue (`GameplayStatics.GetPlayerController` 0))
  (`self.OnSkillIcon`)
  (`self.CheckAltarOnChip`)
  (`self.CheckTimeOut`)
  (if (`self.isEnemyWin`)
    ;[1 1 1] On Enemy Win UI
    (if (`|EnumEquality` (`self.GetRemoteRole` (`self.GetOwner`)) "ROLE_Authority")
      (`Widget.SetVisibility` (`self.EnemyWinRef`) "Visible")
      (`WidgetBlueprintLibrary.SetInputMode_UIOnlyEx` _returnvalue null)
      (set `PlayerController.bShowMouseCursor` true _returnvalue))))

(event `checkEnemyWin`
  ;[1 1 1] Comment
  (set `self.isEnemyWin` true))

(event `CheckTimeOut`
  (bind _vrgamestatebase (`self.vrGameStateBase`))
  ;[1 1 1] Comment
  (`/Engine/EditorBlueprintResources/StandardMacros.IsValid` _vrgamestatebase
    (:`Is Valid`
      (if (`VRGameStateBase.isTimeOut` _vrgamestatebase)
        (set `self.isEnemyWin` true)))))

(event `FirstSkillOn`
  ;[1 1 1] Check Active Skill / C++
  (if (`self.activeFirstSkill`)
    (`/Engine/EditorBlueprintResources/StandardMacros.DoOnce` false
      (:`Completed`
        (`KismetSystemLibrary.PrintString` "FirstON!!!")))))

(event `SecondSkillOn`
  ;[1 1 1] Check Active Skill / C++
  (if (`self.activeSecondSkill`)
    (`/Engine/EditorBlueprintResources/StandardMacros.DoOnce` false
      (:`Completed`
        (`KismetSystemLibrary.PrintString` "SecondON!!!")))))

(event `self.CapsuleComponent.OnComponentBeginOverlap`
  (params (OverlappedComponent :type "PrimitiveComponent Object Reference") (OtherActor :type "Actor Object Reference") (OtherComp :type "PrimitiveComponent Object Reference") (OtherBodyIndex :type Integer) (bFromSweep :type Boolean) (SweepResult :type "HitResult Structure (by ref)"))
  (bind _ashide_player (cast `HidePlayer` OtherActor))
  (set `self.playerChar` _ashide_player))

(event `ThirdSkillOn`
  ;[1 1 1] Check Active Skill / C++
  (if (`self.activeThirdSkill`)
    (`/Engine/EditorBlueprintResources/StandardMacros.DoOnce` false
      (:`Completed`
        (`KismetSystemLibrary.PrintString` "ThirdON!!!")))))

(event `CheckSkillTime`
  ;[1 1 1] Check Active Skill / C++
  (`self.FirstSkillOn`)
  (`self.SecondSkillOn`)
  (`self.ThirdSkillOn`))

(event `self.CapsuleComponent.OnComponentEndOverlap`
  (params (OverlappedComponent :type "PrimitiveComponent Object Reference") (OtherActor :type "Actor Object Reference") (OtherComp :type "PrimitiveComponent Object Reference") (OtherBodyIndex :type Integer))
  (set `self.playerChar` null))

(event `self.handSphereColl.OnComponentBeginOverlap`
  (params (OverlappedComponent :type "PrimitiveComponent Object Reference") (OtherActor :type "Actor Object Reference") (OtherComp :type "PrimitiveComponent Object Reference") (OtherBodyIndex :type Integer) (bFromSweep :type Boolean) (SweepResult :type "HitResult Structure (by ref)")))

(fn `UserConstructionScript`)