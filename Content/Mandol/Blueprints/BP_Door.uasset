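; BP_Door is a door actor that detects players and enemies at its Cube component, with no opening logic in this graph.
; Begin overlap branches on Player or Enemy tags, casts to cache references and sets presence flags; IsEnemy requires both chained enemy casts to succeed.
; End overlap clears player state, but for enemies only resets EnemyOpenTime, leaving their clearing nodes unconnected.
; Debug prints trace these overlaps.
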(event `self.ReceiveTick`
  (params (DeltaSeconds :type "Float (single-precision)")))

(event `self.Cube.OnComponentBeginOverlap`
  (params (OverlappedComponent :type "PrimitiveComponent Object Reference") (OtherActor :type "Actor Object Reference") (OtherComp :type "PrimitiveComponent Object Reference") (OtherBodyIndex :type Integer) (bFromSweep :type Boolean) (SweepResult :type "HitResult Structure (by ref)"))
  (if (`self.ActorHasTag` OtherActor "Player")
    (bind _asbp_test_player (cast `/Game/Mandol/Blueprints/BP_TestPlayer` OtherActor))
    (set `self.Test PlayerRef` _asbp_test_player)
    (set `self.IsPlayer` true)
    (`KismetSystemLibrary.PrintString` "Player Tag")
    (elif (`self.ActorHasTag` OtherActor "Enemy")
      (bind _asbp_test_enemy (cast `/Game/Mandol/Blueprints/BP_TestEnemy` OtherActor))
      (set `self.Test EnemyRef` _asbp_test_enemy)
      (bind _asbp_vrenemy_player (cast `/Game/Mandol/Blueprints/BP_VREnemyPlayer` OtherActor))
      (set `self.VREnemyRef` _asbp_vrenemy_player)
      (set `self.IsEnemy` true)
      (`KismetSystemLibrary.PrintString` "Enemy Tag"))))

(event `self.Cube.OnComponentEndOverlap`
  (params (OverlappedComponent :type "PrimitiveComponent Object Reference") (OtherActor :type "Actor Object Reference") (OtherComp :type "PrimitiveComponent Object Reference") (OtherBodyIndex :type Integer))
  (if (`self.ActorHasTag` OtherActor "Player")
    (set `self.Test PlayerRef` null)
    (set `self.IsPlayer` false)
    (`KismetSystemLibrary.PrintString` "Player Out")
    (elif (`self.ActorHasTag` OtherActor "Enemy")
      (bind _output_get (set `self.EnemyOpenTime` 5.0))
      (`KismetSystemLibrary.PrintString` (`KismetStringLibrary.Conv_DoubleToString` _output_get)))))

(fn `UserConstructionScript`)