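; BP_CableStart is a cable actor whose end can be re-attached to a new end point.
; A custom event attaches the cable end to NewEndStaticMesh and applies BoneWeightMaterial to that mesh and the cable.
; The end sphere's overlap only prints the other actor's name.
; Disconnected leftover logic would attach the cable to BP_HidePlayer's right VR controller on grab and snap it to a sphere on release.
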(event `self.ReceiveTick`
  (params (DeltaSeconds :type "Float (single-precision)")))

(event `CustomEvent`
  (bind _newendstaticmesh (`self.NewEndStaticMesh`))
  (`CableComponent.SetAttachEndToComponent` (`self.CableComponent`) _newendstaticmesh "None")
  (if true
    (`PrimitiveComponent.SetMaterial` _newendstaticmesh 0 "/Engine/EngineDebugMaterials/BoneWeightMaterial.BoneWeightMaterial")
    (`PrimitiveComponent.SetMaterial` (`self.CableComponent`) 0 "/Engine/EngineDebugMaterials/BoneWeightMaterial.BoneWeightMaterial")))

(event `self.NewEndSphereCollision.OnComponentBeginOverlap`
  (params (OverlappedComponent :type "PrimitiveComponent Object Reference") (OtherActor :type "Actor Object Reference") (OtherComp :type "PrimitiveComponent Object Reference") (OtherBodyIndex :type Integer) (bFromSweep :type Boolean) (SweepResult :type "HitResult Structure (by ref)")))

(event `self.EndSphereCollision.OnComponentBeginOverlap`
  (params (OverlappedComponent :type "PrimitiveComponent Object Reference") (OtherActor :type "Actor Object Reference") (OtherComp :type "PrimitiveComponent Object Reference") (OtherBodyIndex :type Integer) (bFromSweep :type Boolean) (SweepResult :type "HitResult Structure (by ref)"))
  (`KismetSystemLibrary.PrintString` (`KismetSystemLibrary.GetDisplayName` OtherActor)))

(fn `UserConstructionScript`)