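; BP_HidePlayer is a VR player Blueprint with a body mesh, two hand controllers, a menu widget and two widget interaction pointers.
; Each tick it passes camera and controller world transforms to ABP_HideyPlayer to drive the body's head and hands.
; The menu input shows the widget and enables the pointers' debug display, which starts off at BeginPlay.
; Tick also unconditionally keeps both pointers visible, and a leader-pose call is left unconnected.
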(event `self.ReceiveBeginPlay`
  (set `WidgetInteractionComponent.bShowDebug` false (`self.WidgetInteraction`))
  (set `WidgetInteractionComponent.bShowDebug` false (`self.WidgetInteraction1`)))

(event `EnhancedInput|/Game/JH/JH_Input/Action/IA_Menu`
  (params (ActionValue :type Boolean) (ElapsedSeconds :type "Float (double-precision)") (TriggeredSeconds :type "Float (double-precision)") (InputAction :type "InputAction Object Reference" :default "/Game/JH/JH_Input/Action/IA_Menu.IA_Menu"))
  (:`Triggered`
    (`SceneComponent.SetVisibility` (`self.Widget`) true false)
    (set `WidgetInteractionComponent.bShowDebug` true (`self.WidgetInteraction`))
    (set `WidgetInteractionComponent.bShowDebug` true (`self.WidgetInteraction1`))))

(event `self.ReceiveTick`
  (params (DeltaSeconds :type "Float (single-precision)"))
  (bind _asabp_hidey_player (cast `/Game/JH/Animation/ABP_HideyPlayer` (`SkeletalMeshComponent.GetAnimInstance` (`self.Mesh`))))
  (set `/Game/JH/Animation/ABP_HideyPlayer.In Head Transform World` (`SceneComponent.K2_GetComponentToWorld` (`self.CameraComponent`)) _asabp_hidey_player)
  (set `/Game/JH/Animation/ABP_HideyPlayer.In Left Hand Transform World` (`SceneComponent.K2_GetComponentToWorld` (`self.LeftController`)) _asabp_hidey_player)
  (set `/Game/JH/Animation/ABP_HideyPlayer.In Right Hand Transform World` (`SceneComponent.K2_GetComponentToWorld` (`self.RightController`)) _asabp_hidey_player)
  (set `self.OnWidget?` (`self.OnWidget?`))
  (if true
    (`SceneComponent.SetVisibility` (`self.WidgetInteraction`) true false)
    (`SceneComponent.SetVisibility` (`self.WidgetInteraction1`) true false)))

(fn `UserConstructionScript`)