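; BP_HidePlayer1 is a VR player Blueprint that drives an animated body mesh from tracked devices.
; Each Tick it casts the mesh's anim instance to ABP_HideyPlayer1 and passes it the world transforms of the camera and both motion controllers as head and hand inputs.
; The construction script is empty, and an unconnected SetLeaderPoseComponent node never runs.
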(event `self.ReceiveTick`
  (params (DeltaSeconds :type "Float (single-precision)"))
  (bind _asabp_hidey_player_1 (cast `/Game/JH/Animation/ABP_HideyPlayer1` (`SkeletalMeshComponent.GetAnimInstance` (`self.Mesh`))))
  (set `/Game/JH/Animation/ABP_HideyPlayer1.In Head Transform World` (`SceneComponent.K2_GetComponentToWorld` (`self.CameraComponent`)) _asabp_hidey_player_1)
  (set `/Game/JH/Animation/ABP_HideyPlayer1.In Left Hand Transform World` (`SceneComponent.K2_GetComponentToWorld` (`self.LeftController`)) _asabp_hidey_player_1)
  (set `/Game/JH/Animation/ABP_HideyPlayer1.In Right Hand Transform World` (`SceneComponent.K2_GetComponentToWorld` (`self.RightController`)) _asabp_hidey_player_1))

(fn `UserConstructionScript`)