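; An interactive duct that swings open after the player's hand touches it.
; An overlap of its box by an actor tagged PlayerHand waits two seconds, sets the state to Open and shows the WBP_Duct widget.
; Tick polls that state to play or reverse a timeline that lerps the root's relative rotation toward a 90-degree angle.
; Nothing in this graph sets the state back to Close.
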(event `self.ReceiveTick`
  (params (DeltaSeconds :type "Float (single-precision)"))
  (switch `/Game/NSE/Blueprints/EDuctState` (`self.DuctState`)
    (:`NewEnumerator1`
      (bind (_direction _ductfloat) (`Timeline|OpenDoorTimeLine` :!label _label)
        (:`Update`
          (`SceneComponent.K2_SetRelativeRotation` (`self.root`) (`KismetMathLibrary.RLerp` (struct) (struct :`Yaw` 90.0) _ductfloat) false false))))
    (:`NewEnumerator2`
      (goto _label :!via `Reverse`))))

(event `self.Box.OnComponentBeginOverlap`
  (params (OverlappedComponent :type "PrimitiveComponent Object Reference") (OtherActor :type "Actor Object Reference") (OtherComp :type "PrimitiveComponent Object Reference") (OtherBodyIndex :type Integer) (bFromSweep :type Boolean) (SweepResult :type "HitResult Structure (by ref)"))
  (if (`self.ActorHasTag` OtherActor "PlayerHand")
    (`KismetSystemLibrary.Delay` 2.0)
    (set `self.DuctState` "NewEnumerator1")
    (bind _returnvalue (`|CreateWidget` "/Game/NSE/UI/WBP_Duct.WBP_Duct_C"))
    (`UserWidget.AddToViewport` _returnvalue 0)))

(fn `UserConstructionScript`)