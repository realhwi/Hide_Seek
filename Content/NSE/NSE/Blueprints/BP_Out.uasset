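; BP_Out is a Blueprint that detects the player's hand in a trigger box, apparently as part of a quiz success check.
; Overlap by a component tagged PlayerHand starts a timer to SucQuiz, resets the mesh's material override and prints a debug string.
; Tick applies the M_OutIng material whenever IsSuc is true, but nothing here sets that flag.
; SucQuiz is an empty stub, so the timer currently has no effect.
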(event `self.ReceiveTick`
  (params (DeltaSeconds :type "Float (single-precision)"))
  (if (`self.IsSuc`)
    (`PrimitiveComponent.SetMaterial` (`self.StaticMesh1`) 0 "/Game/NSE/NSE/Materials/M_OutIng.M_OutIng")))

(event `self.Box.OnComponentBeginOverlap`
  (params (OverlappedComponent :type "PrimitiveComponent Object Reference") (OtherActor :type "Actor Object Reference") (OtherComp :type "PrimitiveComponent Object Reference") (OtherBodyIndex :type Integer) (bFromSweep :type Boolean) (SweepResult :type "HitResult Structure (by ref)"))
  (if (`ActorComponent.ComponentHasTag` OtherComp "PlayerHand")
    (`KismetSystemLibrary.K2_SetTimer` null "SucQuiz" 3.0)
    (`PrimitiveComponent.SetMaterial` (`self.StaticMesh1`) 0 null)
    (`KismetSystemLibrary.PrintString` "Hello")))

(fn `SucQuiz`)

(fn `UserConstructionScript`)