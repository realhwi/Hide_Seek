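; Tag-machine door actor with two sliding panels that player and enemy hands open by staying in the front trigger.
; Front overlap starts an Open timer, longer for enemies on a locked door; leaving cancels it and closes an opened door.
; A player hand entering the back trigger starts a Locked timer.
; State changes enable Tick, which recolours the Cube's dynamic material and plays or reverses two door timelines.
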(event `self.ReceiveBeginPlay`
  (`self.SetActorTickEnabled` false))

(event `self.ReceiveTick`
  (params (DeltaSeconds :type "Float (single-precision)"))
  (bind _cube (`self.Cube`))
  (bind _returnvalue (`PrimitiveComponent.CreateDynamicMaterialInstance` _cube 0 (`PrimitiveComponent.GetMaterial` _cube 0) "None"))
  (bind _output_get (set `self.Mat` _returnvalue))
  (`PrimitiveComponent.SetMaterial` (`self.Cube`) 0 _output_get)
  (switch `/Game/NSE/Blueprints/EDoorState` (`self.DoorState`)
    (:`NewEnumerator1`
      (`MaterialInstanceDynamic.SetVectorParameterValue` (`self.Mat`) "Color" (struct :`G` 1.0 :`B` 0.221756 :`A` 1.0))
      (if (`self.IsOpen`)
        (`|ExecutionSequence`
          (:`then_0`
            ;[1 1 1] 문 Open
            (bind (_direction _doorfloat) (`Timeline|OpenedDoorTimeLine` :!label _label)
              (:`Update`
                (`SceneComponent.K2_SetRelativeLocation` (`self.RightDoor`) (`KismetMathLibrary.VLerp` (0.0 24.0 0.0) (0.0 200.0 0.0) _doorfloat) false false)
                (set `self.IsOpen` false)
                (`self.SetActorTickEnabled` false))))
          (:`then_1`
            ;[1 1 1] 문 Open
            (bind (_direction_2 _doorfloat_2) (`Timeline|Timeline` :!label _label_2)
              (:`Update`
                (`SceneComponent.K2_SetRelativeLocation` (`self.LeftDoor`) (`KismetMathLibrary.VLerp` (0.0 -151.0 0.0) (0.0 -320.0 0.0) _doorfloat_2) false false)
                (set `self.IsOpen` false)
                (`self.SetActorTickEnabled` false)))))))
    (:`NewEnumerator2`
      (`MaterialInstanceDynamic.SetVectorParameterValue` (`self.Mat`) "Color" (struct :`G` 1.0 :`B` 0.221756 :`A` 1.0))
      (`|ExecutionSequence`
        (:`then_0`
          (goto _label :!via `Reverse`))
        (:`then_1`
          (goto _label_2 :!via `Reverse`))))
    (:`NewEnumerator3`
      (`MaterialInstanceDynamic.SetVectorParameterValue` (`self.Mat`) "Color" (struct :`R` 1.0 :`B` 0.810636 :`A` 1.0)))))

(event `self.FrontCollision.OnComponentBeginOverlap`
  (params (OverlappedComponent :type "PrimitiveComponent Object Reference") (OtherActor :type "Actor Object Reference") (OtherComp :type "PrimitiveComponent Object Reference") (OtherBodyIndex :type Integer) (bFromSweep :type Boolean) (SweepResult :type "HitResult Structure (by ref)"))
  (`|ExecutionSequence`
    (:`then_0`
      ;[1 1 1] Player_Open
      (if (`self.ActorHasTag` OtherActor "PlayerHand")
        (`KismetSystemLibrary.K2_SetTimer` null "Open" 3.0)))
    (:`then_1`
      ;[1 1 1] Enemy_Open
      (if (`self.ActorHasTag` OtherActor "EnemyHand")
        (switch `/Game/NSE/Blueprints/EDoorState` (`self.DoorState`)
          (:`NewEnumerator0`
            _)
          (:`NewEnumerator2`
            _))
        (`KismetSystemLibrary.K2_SetTimer` null "Open" 3.0)))
    (:`then_2`
      ;[1 1 1] Enemy_Open(Locked)
      (if (`self.ActorHasTag` OtherActor "EnemyHand")
        (switch `/Game/NSE/Blueprints/EDoorState` (`self.DoorState`)
          (:`NewEnumerator3`
            (`KismetSystemLibrary.K2_SetTimer` null "Open" 10.0)
            (`KismetSystemLibrary.PrintString` "Locked")))))))

(event `self.FrontCollision.OnComponentEndOverlap`
  (params (OverlappedComponent :type "PrimitiveComponent Object Reference") (OtherActor :type "Actor Object Reference") (OtherComp :type "PrimitiveComponent Object Reference") (OtherBodyIndex :type Integer))
  ;[1 1 1] 타임 리셋
  (`KismetSystemLibrary.K2_ClearTimer` null "Open")
  (switch `/Game/NSE/Blueprints/EDoorState` (`self.DoorState`)
    (:`NewEnumerator1`
      (set `self.DoorState` "NewEnumerator2")
      (`self.SetActorTickEnabled` true))))

(event `self.BackCollision.OnComponentBeginOverlap`
  (params (OverlappedComponent :type "PrimitiveComponent Object Reference") (OtherActor :type "Actor Object Reference") (OtherComp :type "PrimitiveComponent Object Reference") (OtherBodyIndex :type Integer) (bFromSweep :type Boolean) (SweepResult :type "HitResult Structure (by ref)"))
  ;[1 1 1] Player_Lock
  (if (`self.ActorHasTag` OtherActor "PlayerHand")
    (`KismetSystemLibrary.K2_SetTimer` null "Locked" 3.0)
    (`KismetSystemLibrary.PrintString` "Locked")))

(fn `Locked`
  (set `self.DoorState` "NewEnumerator3")
  (`self.SetActorTickEnabled` true))

(fn `Open`
  (set `self.DoorState` "NewEnumerator1")
  (set `self.IsOpen` true)
  (`self.SetActorTickEnabled` true))

(fn `Opened_Lock`
  (set `self.DoorState` "NewEnumerator1")
  (set `self.IsOpen` true)
  (`self.SetActorTickEnabled` true))

(fn `UserConstructionScript`)