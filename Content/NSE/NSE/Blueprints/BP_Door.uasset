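; BP_Door is a sliding door that player and enemy hands open by staying in its front collision, and the player can lock from the back.
; Overlaps start named timers that set DoorState, with a longer delay for enemies at a locked door.
; Leaving the front cancels the open timer and closes an opened door.
; Tick, enabled on state changes, plays or reverses a timeline that lerps the door sideways.
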(event `self.ReceiveBeginPlay`
  (`self.SetActorTickEnabled` false))

(event `self.ReceiveTick`
  (params (DeltaSeconds :type "Float (single-precision)"))
  (switch `/Game/NSE/Blueprints/EDoorState` (`self.DoorState`)
    (:`NewEnumerator1`
      (if (`self.IsOpen`)
        ;[1 1 1] 문 Open
        (bind (_direction _doorfloat) (`Timeline|OpenedDoorTimeLine` :!via `PlayFromStart` :!label _label)
          (:`Update`
            (`SceneComponent.K2_SetRelativeLocation` (`self.Door`) (`KismetMathLibrary.VLerp` (0.0 0.0 0.0) (0.0 130.0 0.0) _doorfloat) false false)
            (set `self.IsOpen` false)
            (`self.SetActorTickEnabled` false)))))
    (:`NewEnumerator2`
      (goto _label :!via `Reverse`))))

(event `self.FrontCollision.OnComponentBeginOverlap`
  (params (OverlappedComponent :type "PrimitiveComponent Object Reference") (OtherActor :type "Actor Object Reference") (OtherComp :type "PrimitiveComponent Object Reference") (OtherBodyIndex :type Integer) (bFromSweep :type Boolean) (SweepResult :type "HitResult Structure (by ref)"))
  (`|ExecutionSequence`
    (:`then_0`
      ;[1 1 1] Player_Open
      (if (`self.ActorHasTag` OtherActor "PlayerHand")
        (`KismetSystemLibrary.K2_SetTimer` null "Open" 3.0)))
    (:`then_1`
      ;[1 1 1] Enemy_Open
      (if (`self.ActorHasTag` OtherActor "EnemyHand")
        (switch `/Game/NSE/Blueprints/EDoorState` (`self.DoorState`)
          (:`NewEnumerator0`
            _)
          (:`NewEnumerator2`
            _))
        (`KismetSystemLibrary.K2_SetTimer` null "Open" 3.0)))
    (:`then_2`
      ;[1 1 1] Enemy_Open(Locked)
      (if (`self.ActorHasTag` OtherActor "EnemyHand")
        (switch `/Game/NSE/Blueprints/EDoorState` (`self.DoorState`)
          (:`NewEnumerator3`
            (`KismetSystemLibrary.K2_SetTimer` null "Open" 10.0)
            (`KismetSystemLibrary.PrintString` "Locked")))))))

(event `self.FrontCollision.OnComponentEndOverlap`
  (params (OverlappedComponent :type "PrimitiveComponent Object Reference") (OtherActor :type "Actor Object Reference") (OtherComp :type "PrimitiveComponent Object Reference") (OtherBodyIndex :type Integer))
  ;[1 1 1] 타임 리셋
  (`KismetSystemLibrary.K2_ClearTimer` null "Open")
  (switch `/Game/NSE/Blueprints/EDoorState` (`self.DoorState`)
    (:`NewEnumerator1`
      (set `self.DoorState` "NewEnumerator2")
      (`self.SetActorTickEnabled` true))))

(event `self.BackCollision.OnComponentBeginOverlap`
  (params (OverlappedComponent :type "PrimitiveComponent Object Reference") (OtherActor :type "Actor Object Reference") (OtherComp :type "PrimitiveComponent Object Reference") (OtherBodyIndex :type Integer) (bFromSweep :type Boolean) (SweepResult :type "HitResult Structure (by ref)"))
  ;[1 1 1] Player_Lock
  (if (`self.ActorHasTag` OtherActor "PlayerHand")
    (`KismetSystemLibrary.K2_SetTimer` null "Locked" 3.0)
    (`KismetSystemLibrary.PrintString` "Locked")))

(fn `Locked`
  (set `self.DoorState` "NewEnumerator3")
  (`self.SetActorTickEnabled` true))

(fn `Open`
  (set `self.DoorState` "NewEnumerator1")
  (set `self.IsOpen` true)
  (`self.SetActorTickEnabled` true))

(fn `Opened_Lock`
  (set `self.DoorState` "NewEnumerator1")
  (set `self.IsOpen` true)
  (`self.SetActorTickEnabled` true))

(fn `UserConstructionScript`)