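; BP_Puzzle is a rotation puzzle that drives a linked Door, with Q rotating its StaticMesh in yaw by RotateValue.
; After each turn, CheckData compares the yaw to the Code entry within a tolerance and stores the result in CodeISGood.
; Any false entry opens the Door, otherwise it closes, and a dynamic material recolors the Ring to match.
; Both RotateLeft branches rotate identically, and the interact events are empty.
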(event `Key|Q`
  (params (Key :type "Key Structure"))
  (:`Pressed`
    (`self.Rotate` (`self.StaticMesh`) (`self.Rotate Left`))))

(event `self.InteractWithPuzzle`
  (params (Component :type "PrimitiveComponent Object Reference") (RotateLeft :type Boolean)))

(event `self.OnTriggerInteract`
  (params (Player :type "HidePlayer Object Reference")))

(fn `Check Data`
  (params (Component :type "PrimitiveComponent Object Reference"))
  (locals (SelectMesh :type Integer) (LocalFailed :type Boolean))
  (bind (_relativerotation_roll _relativerotation_pitch _relativerotation_yaw) (`KismetMathLibrary.BreakRotator` (`SceneComponent.RelativeRotation` Component)))
  (bind _ring (`self.ring`))
  (bind _ring_2 (`self.ring`))
  (bind _door (`self.Door`))
  (if (== Component (`self.StaticMesh`))
    (set `local.SelectMesh` 0)
    (`KismetArrayLibrary.Array_Set` (`self.CodeISGood`) (`local.SelectMesh`) (`KismetMathLibrary.NearlyEqual_FloatFloat` (`|GetArrayItem` (`self.Code`) (`local.SelectMesh`)) _relativerotation_yaw 10.0))
    (for _array_element (`self.CodeISGood`)
      (if (not _array_element)
        (set `local.LocalFailed` true)
        (break)))
    (if (`local.LocalFailed`)
      (`KismetSystemLibrary.PrintString` "Open")
      (bind _returnvalue (`PrimitiveComponent.CreateDynamicMaterialInstance` _ring_2 0 (`PrimitiveComponent.GetMaterial` _ring_2 0) "None"))
      (bind _output_get (set `self.NewVar` _returnvalue))
      (`PrimitiveComponent.SetMaterial` (`self.ring`) 0 _output_get)
      (`MaterialInstanceDynamic.SetVectorParameterValue` (`self.NewVar`) "Color" (struct :`R` 0.818894 :`B` 1.0 :`A` 1.0))
      (`/Game/NSE/Blueprints/ItemBox/BP_BoxDoor.Open` _door)
      (else
        (`KismetSystemLibrary.PrintString` "Close")
        (bind _returnvalue_2 (`PrimitiveComponent.CreateDynamicMaterialInstance` _ring 0 (`PrimitiveComponent.GetMaterial` _ring 0) "None"))
        (bind _output_get_2 (set `self.NewVar` _returnvalue_2))
        (`PrimitiveComponent.SetMaterial` (`self.ring`) 0 _output_get_2)
        (`MaterialInstanceDynamic.SetVectorParameterValue` (`self.NewVar`) "Color" (struct :`G` 0.957452 :`B` 1.0 :`A` 1.0))
        (`/Game/NSE/Blueprints/ItemBox/BP_BoxDoor.Close` _door)))))

(fn `Rotate`
  (params (Component :type "PrimitiveComponent Object Reference") (RotateLeft :type Boolean))
  (if RotateLeft
    (`SceneComponent.K2_AddRelativeRotation` Component (`KismetMathLibrary.MakeRotator` 0.0 0.0 (`self.RotateValue`)) false false)
    (else
      (`SceneComponent.K2_AddRelativeRotation` Component (`KismetMathLibrary.MakeRotator` 0.0 0.0 (`self.RotateValue`)) false false)))
  (`KismetSystemLibrary.PrintString` (`KismetStringLibrary.Conv_RotatorToString` (`SceneComponent.RelativeRotation` Component)))
  (`self.Check Data` Component))

(fn `UserConstructionScript`)