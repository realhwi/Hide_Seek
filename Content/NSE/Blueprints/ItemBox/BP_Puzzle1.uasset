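; BP_Puzzle1 is an interactable rotation puzzle tied to a Door and a Ring indicator.
; Each trigger interaction yaws StaticMesh by RotateValue (same in both RotateLeft branches), then checks it against the first Code entry with a tolerance.
; Any false CodeISGood entry closes the Door and recolors the Ring cyan through a dynamic material.
; The door-opening, purple-ring success logic is present but disconnected, so solving the puzzle triggers nothing here.
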(event `self.OnTriggerInteract`
  (params (Player :type "HidePlayer Object Reference"))
  (`self.Rotate` (`self.StaticMesh`) (`self.Rotate Left`)))

(event `EnhancedInput|/Game/JH/JH_Input/Action/IA_Trigger`
  (params (ActionValue :type "Float (double-precision)") (ElapsedSeconds :type "Float (double-precision)") (TriggeredSeconds :type "Float (double-precision)") (InputAction :type "InputAction Object Reference" :default "/Game/JH/JH_Input/Action/IA_Trigger.IA_Trigger")))

(fn `Check Data`
  (params (Component :type "PrimitiveComponent Object Reference"))
  (locals (SelectMesh :type Integer) (LocalFailed :type Boolean))
  (bind (_relativerotation_roll _relativerotation_pitch _relativerotation_yaw) (`KismetMathLibrary.BreakRotator` (`SceneComponent.RelativeRotation` Component)))
  (bind _ring (`self.ring`))
  (if (== Component (`self.StaticMesh`))
    (set `local.SelectMesh` 0)
    (`KismetArrayLibrary.Array_Set` (`self.CodeISGood`) (`local.SelectMesh`) (`KismetMathLibrary.NearlyEqual_FloatFloat` (`|GetArrayItem` (`self.Code`) (`local.SelectMesh`)) _relativerotation_yaw 10.0))
    (for _array_element (`self.CodeISGood`)
      (if (not _array_element)
        (set `local.LocalFailed` true)
        (break)))
    (if (`local.LocalFailed`)
      (`/Game/NSE/Blueprints/ItemBox/BP_BoxDoor.Close` (`self.Door`))
      (bind _returnvalue (`PrimitiveComponent.CreateDynamicMaterialInstance` _ring 0 (`PrimitiveComponent.GetMaterial` _ring 0) "None"))
      (bind _output_get (set `self.NewVar` _returnvalue))
      (`PrimitiveComponent.SetMaterial` (`self.ring`) 0 _output_get)
      (`MaterialInstanceDynamic.SetVectorParameterValue` (`self.NewVar`) "Color" (struct :`G` 0.957452 :`B` 1.0 :`A` 1.0)))))

(fn `Rotate`
  (params (Component :type "PrimitiveComponent Object Reference") (RotateLeft :type Boolean))
  (if RotateLeft
    (`SceneComponent.K2_AddRelativeRotation` Component (`KismetMathLibrary.MakeRotator` 0.0 0.0 (`self.RotateValue`)) false false)
    (else
      (`SceneComponent.K2_AddRelativeRotation` Component (`KismetMathLibrary.MakeRotator` 0.0 0.0 (`self.RotateValue`)) false false)))
  (`KismetSystemLibrary.PrintString` (`KismetStringLibrary.Conv_RotatorToString` (`SceneComponent.RelativeRotation` Component)))
  (`self.Check Data` Component))

(fn `UserConstructionScript`)