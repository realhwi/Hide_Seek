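; BP_BoxDoor is a hinged door Blueprint, likely for an item box, that swings open and closed through exposed Open and Close events.
; Open plays a timeline from the start, lerping the Sphere component's relative roll from 0 to 90 degrees and setting IsOpen with debug prints.
; Close reverses the same timeline; IsOpen is never cleared, and branches checking it are unconnected.
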(event `Open`
  (`KismetSystemLibrary.PrintString` "openopemn")
  (bind (_direction _doorfloat) (`Timeline|OpenTimeline` :!via `PlayFromStart` :!label _label)
    (:`Update`
      (`SceneComponent.K2_SetRelativeRotation` (`self.Sphere`) (`KismetMathLibrary.MakeRotator` (`KismetMathLibrary.Lerp` 0.0 90.0 _doorfloat)) false false)
      (`KismetSystemLibrary.PrintString` "OpenBox")
      (set `self.Is Open` true))))

(event `Close`
  (goto _label :!via `Reverse`))

(fn `UserConstructionScript`)