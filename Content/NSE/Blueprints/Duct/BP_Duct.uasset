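; BP_Duct is a duct whose door swings open when a component tagged PlayerHand touches it.
; Overlapping the Box sets DuctState to Open, and leaving CloseCollision sets it to Close after a short delay.
; Tick checks that state every frame and plays or reverses a Timeline, whose float track lerps the Root's relative rotation through a quarter turn.
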(event `self.ReceiveTick`
  (params (DeltaSeconds :type "Float (single-precision)"))
  (switch `/Game/NSE/Blueprints/Duct/EDuctState` (`self.DuctState`)
    (:`NewEnumerator1`
      (bind (_direction _doorfloat) (`Timeline|Timeline` :!label _label)
        (:`Update`
          (`SceneComponent.K2_SetRelativeRotation` (`self.root`) (`KismetMathLibrary.RLerp` (struct) (struct :`Yaw` -90.0) _doorfloat) false false))))
    (:`NewEnumerator2`
      (goto _label :!via `Reverse`))))

(event `self.Box.OnComponentBeginOverlap`
  (params (OverlappedComponent :type "PrimitiveComponent Object Reference") (OtherActor :type "Actor Object Reference") (OtherComp :type "PrimitiveComponent Object Reference") (OtherBodyIndex :type Integer) (bFromSweep :type Boolean) (SweepResult :type "HitResult Structure (by ref)"))
  (if (`ActorComponent.ComponentHasTag` OtherComp "PlayerHand")
    (set `self.DuctState` "NewEnumerator1")))

(event `self.CloseCollision.OnComponentEndOverlap`
  (params (OverlappedComponent :type "PrimitiveComponent Object Reference") (OtherActor :type "Actor Object Reference") (OtherComp :type "PrimitiveComponent Object Reference") (OtherBodyIndex :type Integer))
  (if (`ActorComponent.ComponentHasTag` OtherComp "PlayerHand")
    (`KismetSystemLibrary.Delay` 1.0)
    (set `self.DuctState` "NewEnumerator2")))

(fn `UserConstructionScript`)