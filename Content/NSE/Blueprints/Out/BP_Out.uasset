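; BP_Out is an actor with a Box trigger that drives the state of a Button through a timed hold after a player hand touches it.
; An overlap from a PlayerHand-tagged component while the Button is Active or Loading sets it to Loading and starts a three-second timer.
; The timer calls SucQuiz, which flags OnceB and sets Success if still Loading.
; An Active function returns the Button to Active.
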(event `self.Box.OnComponentBeginOverlap`
  (params (OverlappedComponent :type "PrimitiveComponent Object Reference") (OtherActor :type "Actor Object Reference") (OtherComp :type "PrimitiveComponent Object Reference") (OtherBodyIndex :type Integer) (bFromSweep :type Boolean) (SweepResult :type "HitResult Structure (by ref)"))
  (if (`ActorComponent.ComponentHasTag` OtherComp "PlayerHand")
    (`KismetSystemLibrary.PrintString` "Overlap")
    (switch `/Game/NSE/Blueprints/Out/EOutState` (`/Game/NSE/Blueprints/Out/BP_Button.ButtonState` (`self.Button`))
      (:`NewEnumerator1`
        _)
      (:`NewEnumerator2`
        _))
    (`KismetSystemLibrary.K2_SetTimer` null "SucQuiz" 3.0)
    (set `/Game/NSE/Blueprints/Out/BP_Button.ButtonState` "NewEnumerator2" (`self.Button`))
    (`KismetSystemLibrary.PrintString` "Good")))

(fn `Active`
  (set `/Game/NSE/Blueprints/Out/BP_Button.ButtonState` "NewEnumerator1" (`self.Button`)))

(fn `SucQuiz`
  (bind _button (`self.Button`))
  (switch `/Game/NSE/Blueprints/Out/EOutState` (`/Game/NSE/Blueprints/Out/BP_Button.ButtonState` (`self.Button`))
    (:`NewEnumerator2`
      (set `/Game/NSE/Blueprints/Out/BP_Button.Once_B` true _button)
      (set `/Game/NSE/Blueprints/Out/BP_Button.ButtonState` "NewEnumerator3" _button))))

(fn `UserConstructionScript`)