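; BP_Button is a button actor that shows its current state through the material on its static mesh.
; Every Tick it switches on ButtonState and applies a matching material for Active, Loading or Success.
; The Success branch is gated by the OnceB flag, so its material change and SucCount increment run only while that flag is set, then clear it.
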(event `self.ReceiveTick`
  (params (DeltaSeconds :type "Float (single-precision)"))
  (switch `/Game/NSE/Blueprints/Out/EOutState` (`self.ButtonState`)
    (:`NewEnumerator1`
      (`PrimitiveComponent.SetMaterial` (`self.StaticMesh`) 0 "/Game/NSE/Materials/M_OutIng.M_OutIng"))
    (:`NewEnumerator2`
      (`PrimitiveComponent.SetMaterial` (`self.StaticMesh`) 0 "/Game/NSE/Materials/M_OutIng1.M_OutIng1"))
    (:`NewEnumerator3`
      (if (`self.Once_B`)
        (`PrimitiveComponent.SetMaterial` (`self.StaticMesh`) 0 "/Game/NSE/Materials/M_OutSuc.M_OutSuc")
        (set `self.SucCount` (+ (`self.SucCount`) 1))
        (set `self.Once_B` false)))))

(fn `UserConstructionScript`)