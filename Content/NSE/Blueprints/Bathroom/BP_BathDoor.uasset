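; BP_BathDoor is a bathroom door that swings open automatically when a player or enemy hand enters its trigger box.
; Box overlaps from actors tagged PlayerHand or EnemyHand set a door state enum to Open, and leaving sets it to Close after a short delay.
; Tick switches on that state to play or reverse a timeline, whose float drives the Sphere component's relative yaw through a quarter turn.
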(event `self.ReceiveTick`
  (params (DeltaSeconds :type "Float (single-precision)"))
  (switch `/Game/NSE/Blueprints/Bathroom/EBathRoomDoorState` (`self.EBDoorState`)
    (:`NewEnumerator1`
      (bind (_direction _doorfloat) (`Timeline|Timeline` :!label _label)
        (:`Update`
          (`SceneComponent.K2_SetRelativeRotation` (`self.Sphere`) (`KismetMathLibrary.RLerp` (struct) (struct :`Pitch` -90.0) _doorfloat) false false))))
    (:`NewEnumerator2`
      (goto _label :!via `Reverse`))))

(event `self.Box.OnComponentBeginOverlap`
  (params (OverlappedComponent :type "PrimitiveComponent Object Reference") (OtherActor :type "Actor Object Reference") (OtherComp :type "PrimitiveComponent Object Reference") (OtherBodyIndex :type Integer) (bFromSweep :type Boolean) (SweepResult :type "HitResult Structure (by ref)"))
  (if (or (`self.ActorHasTag` OtherActor "PlayerHand") (`self.ActorHasTag` OtherActor "EnemyHand"))
    (set `self.EBDoorState` "NewEnumerator1")))

(event `self.Box.OnComponentEndOverlap`
  (params (OverlappedComponent :type "PrimitiveComponent Object Reference") (OtherActor :type "Actor Object Reference") (OtherComp :type "PrimitiveComponent Object Reference") (OtherBodyIndex :type Integer))
  (if (or (`self.ActorHasTag` OtherActor "PlayerHand") (`self.ActorHasTag` OtherActor "EnemyHand"))
    (`KismetSystemLibrary.Delay` 1.0)
    (set `self.EBDoorState` "NewEnumerator2")))

(fn `UserConstructionScript`)