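; BP_Hide is an interactable actor, apparently a hiding spot, that moves BP_Player in and out of position.
; When a PlayerHand-tagged component touches its Button, it snaps the player to Point, resets the camera offset, adds a WBP_Move widget and shows FX.
; Tick polls that widget's Open flag, then shifts the player along world X with a compensating camera offset and removes the widget.
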(event `self.Button.OnComponentBeginOverlap`
  (params (OverlappedComponent :type "PrimitiveComponent Object Reference") (OtherActor :type "Actor Object Reference") (OtherComp :type "PrimitiveComponent Object Reference") (OtherBodyIndex :type Integer) (bFromSweep :type Boolean) (SweepResult :type "HitResult Structure (by ref)"))
  (bind (_returnvalue_x _returnvalue_y) (`KismetMathLibrary.BreakVector` (`SceneComponent.K2_GetComponentLocation` (`self.Point`))))
  ;[1 1 1 0.5 25] 버튼 누르면
  (if (`ActorComponent.ComponentHasTag` OtherComp "PlayerHand")
    (bind _returnvalue (`GameplayStatics.GetActorOfClass` "/Game/NSE/Blueprints/Player/BP_Player.BP_Player_C"))
    (`SceneComponent.K2_SetRelativeLocation` (`Actor.RootComponent` _returnvalue) (`KismetMathLibrary.MakeVector` _returnvalue_x _returnvalue_y 88.0) false false) ; 플레이어 위치 조정
    (`SceneComponent.K2_SetRelativeLocation` (`/Game/NSE/Blueprints/Player/BP_Player.Camera` _returnvalue) (0.0 0.0 88.0) false false) ; 카메라 위치 조정
    (bind _returnvalue_2 (`|CreateWidget` "/Game/NSE/UI/WBP_Move.WBP_Move_C"))
    (`UserWidget.AddToViewport` _returnvalue_2 0)
    (`SceneComponent.SetVisibility` (`self.FX`) true false)))

(event `self.ReceiveTick`
  (params (DeltaSeconds :type "Float (single-precision)"))
  ;[1 1 1 1 25] Open
  (if (`KismetArrayLibrary.Array_IsValidIndex` (stale _foundwidgets))
    (bind _foundwidgets (`WidgetBlueprintLibrary.GetAllWidgetsOfClass` "/Game/NSE/UI/WBP_Move.WBP_Move_C"))
    (bind _output (`|GetArrayItem` _foundwidgets))
    (if (`/Game/NSE/UI/WBP_Move.Open` _output)
      (bind _returnvalue (`GameplayStatics.GetActorOfClass` "/Game/NSE/Blueprints/Player/BP_Player.BP_Player_C"))
      (bind (_returnvalue_x _returnvalue_y _returnvalue_z) (`KismetMathLibrary.BreakVector` (`SceneComponent.K2_GetComponentLocation` (`Actor.RootComponent` _returnvalue))))
      (`self.K2_SetActorLocation` _returnvalue (`KismetMathLibrary.MakeVector` (+ _returnvalue_x 200.0) _returnvalue_y _returnvalue_z) false false)
      (`SceneComponent.K2_SetRelativeLocation` (`/Game/NSE/Blueprints/Player/BP_Player.Camera` _returnvalue) (-200.0 0.0 88.0) false false)
      (set `/Game/NSE/UI/WBP_Move.Open` false _output)
      (`Widget.RemoveFromParent` _output))))

(fn `UserConstructionScript`)